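; BP_Arrow is an arrow actor that tilts to point at the mouse cursor.
; At BeginPlay it records whether the player controller's yaw is zero to determine the character's facing direction.
; Each tick it traces under the cursor on a custom channel, intended to hit CursorPlane, and computes a look-at pitch to that point.
; Only pitch drives the rotation, mirrored as 180 minus pitch when the initial yaw is non-zero.
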(event EventBeginPlay
  ;[1 0 1] Определение направления персонажа
  (Variables|Default|SetdefoultRotation (== (.yaw (Pawn|GetControlRotation (Game|GetPlayerController 0) :!class /Script/Engine.Controller)) 0.0)))

(event Collision|EventActorBeginOverlap
  (params (OtherActor :type Actor%20Object%20Reference)))

(event EventTick
  (params (DeltaSeconds :type Float%20%28single-precision%29))
  (bind _returnvalue (Transformation|GetActorLocation))
  (bind _returnvalue_2 (Game|GetPlayerController 0))
  (bind _hitresult (Game|Player|GetHitResultUnderCursorbyChannel _returnvalue_2 "TraceTypeQuery3" true))
  (bind _returnvalue_3 (Math|Rotator|FindLookatRotation _returnvalue (.location _hitresult)))
  ;[1 0 1] Поворот к месту пересечения луча MouseCursorTrace и объекта CursorPlane
  (Transformation|SetActorRotation (Math|Rotator|MakeRotator 0.0 (Math|Float|SelectFloat (.pitch _returnvalue_3) (- 1.8e+02 (.pitch _returnvalue_3)) (Variables|Default|GetdefoultRotation)) 0.0)))

(fn ConstructionScript)