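; BP_Camera is the view-target camera that frames Pirat, Delo, Varp and, when present, Pinus on the XZ plane.
; BeginPlay caches actor references, and RefreshPinus copies the Pinus reference from Pirat.
; In auto mode, Tick runs AllFocus, which centers the actor between min/max target positions and derives camera Y distance from their spread.
; A toggle input switches to manual pan and zoom, with pan speed scaled by camera distance.
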(event Input|EnhancedActionEvents|EnhancedInputActionIA_FlipCameraMode
  (params (ActionValue :type Boolean) (ElapsedSeconds :type Float%20%28double-precision%29) (TriggeredSeconds :type Float%20%28double-precision%29) (InputAction :type Input%20Action%20Object%20Reference :default "/Game/inputs/IA_FlipCameraMode.IA_FlipCameraMode"))
  ;[0 1 0] Переключение режима камеры
  (Variables|Default|Setautomode (not (Variables|Default|Getautomode))))

(event Input|EnhancedActionEvents|EnhancedInputActionIA_HorizontalCameraMove
  (params (ActionValue :type Float%20%28double-precision%29) (ElapsedSeconds :type Float%20%28double-precision%29) (TriggeredSeconds :type Float%20%28double-precision%29) (InputAction :type Input%20Action%20Object%20Reference :default "/Game/inputs/IA_HorizontalCameraMove.IA_HorizontalCameraMove"))
  ;[0 1 0] Двжение камеры по горизонтали
  (if (not (Variables|Default|Getautomode))
    (Transformation|AddActorWorldOffset (Math|Vector|MakeVector (* ActionValue (/ (.y (Variables|/Script/Engine.SceneComponent|GetRelativeLocation (Variables|Default|GetCamera))) 5e+01)) 0.0 0.0))))

(event Input|EnhancedActionEvents|EnhancedInputActionIA_VerticalCameraMove
  (params (ActionValue :type Float%20%28double-precision%29) (ElapsedSeconds :type Float%20%28double-precision%29) (TriggeredSeconds :type Float%20%28double-precision%29) (InputAction :type Input%20Action%20Object%20Reference :default "/Game/inputs/IA_VerticalCameraMove.IA_VerticalCameraMove"))
  ;[0 1 0] Движение камеры по вертикали
  (if (not (Variables|Default|Getautomode))
    (Transformation|AddActorWorldOffset (Math|Vector|MakeVector 0.0 0.0 (* ActionValue (/ (.y (Variables|/Script/Engine.SceneComponent|GetRelativeLocation (Variables|Default|GetCamera))) 5e+01))))))

(event Input|EnhancedActionEvents|EnhancedInputActionIA_Zoom
  (params (ActionValue :type Float%20%28double-precision%29) (ElapsedSeconds :type Float%20%28double-precision%29) (TriggeredSeconds :type Float%20%28double-precision%29) (InputAction :type Input%20Action%20Object%20Reference :default "/Game/inputs/IA_Zoom.IA_Zoom"))
  ;[0 1 0] Zoom камеры
  (if (not (Variables|Default|Getautomode))
    (Transformation|AddRelativeLocation (Variables|Default|GetCamera) (Math|Vector|MakeVector 0.0 (* ActionValue -5e+01) 0.0) false false)))

(event EventBeginPlay
  (bind _returnvalue (Game|GetPlayerController 0))
  ;[1 1 0] Привязка камеры и создание указателей на ключевые объекты
  (Utilities|IsValid _returnvalue
    (:Is%20Valid
      (Game|Player|SetViewTargetwithBlend _returnvalue self 0.0 "VTBlend_Linear" 0.0 false)
      (bind _returnvalue_2 (Actor|GetActorOfClass "/Game/objects/pirat/BP_Pirat.BP_Pirat_C"))
      (Variables|Default|Setref_bp_pirat (Utilities|ResolveSoftReference _returnvalue_2))
      (bind _returnvalue_3 (Actor|GetActorOfClass "/Game/objects/delo/BP_Delo.BP_Delo_C"))
      (Variables|Default|Setref_bp_delo (Utilities|ResolveSoftReference _returnvalue_3))
      (bind _returnvalue_4 (Actor|GetActorOfClass "/Game/objects/varp/BP_Varp.BP_Varp_C"))
      (Variables|Default|Setref_bp_varp (Utilities|ResolveSoftReference _returnvalue_4))
      (CallFunction|RefreshPinus))))

(event EventTick
  (params (DeltaSeconds :type Float%20%28single-precision%29))
  ;[0.5 0 1] Исполнение выбранного режима
  (if (Variables|Default|Getautomode)
    (CallFunction|AllFocus)))

(fn ConstructionScript)

(fn AllFocus
  (bind _ref_bp_pirat (Variables|Default|Getref_bp_pirat))
  (bind _ref_bp_delo (Variables|Default|Getref_bp_delo))
  (bind _ref_bp_varp (Variables|Default|Getref_bp_varp))
  (bind _ref_bp_pinus (Variables|Default|Getref_bp_pinus))
  (bind _output (Utilities|ResolveSoftReference _ref_bp_pirat))
  (bind _output_2 (Utilities|ResolveSoftReference _ref_bp_varp))
  (bind _output_3 (Utilities|ResolveSoftReference _ref_bp_delo))
  (bind _output_4 (Utilities|ResolveSoftReference _ref_bp_pinus))
  (bind _returnvalue (Transformation|GetActorLocation _output_4))
  (bind _returnvalue_2 (Transformation|GetActorLocation _output))
  (bind _returnvalue_3 (Transformation|GetActorLocation _output_2))
  (bind _returnvalue_4 (Transformation|GetActorLocation _output_3))
  (bind _returnvalue_5 (Math|Float|Min(Float) (.x _returnvalue_2) (.x _returnvalue_4) (.x _returnvalue_3) (.x _returnvalue)))
  (bind _returnvalue_6 (Math|Float|Max(Float) (.z _returnvalue_2) (.z _returnvalue_4) (.z _returnvalue_3) (.z _returnvalue)))
  (bind _returnvalue_7 (Math|Float|Min(Float) (.z _returnvalue_2) (.z _returnvalue_4) (.z _returnvalue_3) (.z _returnvalue)))
  (bind _returnvalue_8 (Math|Float|Max(Float) (.x _returnvalue_2) (.x _returnvalue_4) (.x _returnvalue_3) (.x _returnvalue)))
  (bind _returnvalue_9 (Math|Float|Min(Float) (.x _returnvalue_2) (.x _returnvalue_4) (.x _returnvalue_3)))
  (bind _returnvalue_10 (Math|Float|Max(Float) (.x _returnvalue_2) (.z _returnvalue_4) (.x _returnvalue_3)))
  (bind _returnvalue_11 (Math|Float|Min(Float) (.z _returnvalue_2) (.z _returnvalue_4) (.z _returnvalue_3)))
  (bind _returnvalue_12 (Math|Float|Max(Float) (.z _returnvalue_2) (.z _returnvalue_4) (.z _returnvalue_3)))
  (bind _returnvalue_13 (- _returnvalue_6 _returnvalue_7))
  (bind _returnvalue_14 (- _returnvalue_12 _returnvalue_11))
  (bind _returnvalue_15 (- _returnvalue_8 _returnvalue_5))
  (bind _returnvalue_16 (- _returnvalue_10 _returnvalue_9))
  (bind _returnvalue_17 (Math|Float|Absolute(Float) _returnvalue_16))
  (bind _returnvalue_18 (Math|Float|Absolute(Float) _returnvalue_14))
  (bind _returnvalue_19 (Math|Float|Absolute(Float) _returnvalue_13))
  (bind _returnvalue_20 (Math|Float|Absolute(Float) _returnvalue_15))
  ;[1 0.2731 0.5816] Определение максимальной дистанции между ключевыми объектами
  ; Расположение камеры посередке, дабы всех было видно
  (if (Variables|/Game/objects/pirat/BP_Pirat.BP_Pirat_C|GetpinusIsCreated _output)
    (Utilities|IsValid _output_4
      (:Is%20Valid
        ;;[0.8069 1 0.4741] Если Pinus существует
        (Transformation|SetActorLocation (Math|Vector|MakeVector (+ _returnvalue_5 (/ _returnvalue_20 2.0)) 0.0 (+ _returnvalue_7 (/ _returnvalue_19 2.0))) false false)
        (Transformation|SetRelativeLocation (Variables|Default|GetCamera) (Math|Vector|MakeVector 0.0 (Math|Float|Max(Float) (* _returnvalue_20 0.625) (* _returnvalue_19 1.0)) 0.0) false false))
      (:Is%20Not%20Valid
        ;;[0.7222 1 0.3846] Если Pinus отвязан
        (Transformation|SetActorLocation (Math|Vector|MakeVector (+ _returnvalue_9 (/ _returnvalue_17 2.0)) 0.0 (+ _returnvalue_11 (/ _returnvalue_18 2.0))) false false :!label _label)
        (Transformation|SetRelativeLocation (Variables|Default|GetCamera) (Math|Vector|MakeVector 0.0 (Math|Float|Max(Float) (* _returnvalue_17 0.625) (* _returnvalue_18 1.0)) 0.0) false false)))
    (else
      (goto _label))))

(fn RefreshPinus
  (Utilities|IsValid (Utilities|ResolveSoftReference (Variables|/Game/objects/pirat/BP_Pirat.BP_Pirat_C|Getref_bp_pinus (Utilities|ResolveSoftReference (Variables|Default|Getref_bp_pirat))))
    (:Is%20Valid
      (Variables|Default|Setref_bp_pinus (Variables|/Game/objects/pirat/BP_Pirat.BP_Pirat_C|Getref_bp_pinus (Utilities|ResolveSoftReference (Variables|Default|Getref_bp_pirat)))))))