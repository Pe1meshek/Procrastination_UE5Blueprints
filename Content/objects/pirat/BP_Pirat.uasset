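; Player-controlled pirate with flipbook animations that spawns, kicks, activates and unbinds Pinus projectiles, and can flip facing.
; Spawning picks the class from the selected index, stores the reference and refreshes BP_Camera.
; The Charge flipbook's playback frame sets kick power, and the kick also fires when it finishes.
; After an attack delay, KickPinus destroys all arrows and impulses Pinus overlapping BoxAttack in X/Z, angled toward the cursor.
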(event OnFinishedPlaying(charge)
  (bind _char (Variables|Default|Getchar))
  (bind _charge (Variables|Default|Getcharge))
  ;[0 1 1] Подготовка Pinus и Pirat к Pinus Kick
  (Audio|Components|Audio|Stop _charge)
  (Rendering|SetVisibility _charge false false)
  (bind _result (Math|Integer|IncrementInt (Class|PaperFlipbookComponent|GetPlaybackPositioninFrames _charge))
    (:%20%20
      (Variables|Default|SetkickPower _result)
      (Sprite|SetFlipbook _char "/Game/objects/pirat/attack.attack")
      (Components|Timeline|PlayfromStart _char)
      (Utilities|FlowControl|Delay 0.4)
      (CallFunction|KickPinus))))

(event OnFinishedPlaying(char)
  (bind _char (Variables|Default|Getchar))
  ;[1 1 1] Цикличность анимаций
  (Sprite|SetFlipbook _char "/Game/objects/pirat/idle.idle")
  (Components|Timeline|PlayfromStart _char))

(event Input|EnhancedActionEvents|EnhancedInputActionIA_CreatePinus
  (params (ActionValue :type Boolean) (ElapsedSeconds :type Float%20%28double-precision%29) (TriggeredSeconds :type Float%20%28double-precision%29) (InputAction :type Input%20Action%20Object%20Reference :default "/Game/inputs/IA_CreatePinus.IA_CreatePinus"))
  ;[0 1 1] Создание Pinus
  (Utilities|IsValid (Utilities|ResolveSoftReference (Variables|Default|Getref_bp_pinus))
    (:Is%20Valid
      (Utilities|IsValid (Variables|/Game/objects/pinus/BP_Pinus.BP_Pinus_C|Getbp_arrow (Utilities|ResolveSoftReference (Variables|Default|Getref_bp_pinus)))
        (:Is%20Valid
          (Actor|DestroyActor (Variables|/Game/objects/pinus/BP_Pinus.BP_Pinus_C|Getbp_arrow (Utilities|ResolveSoftReference (Variables|Default|Getref_bp_pinus)))))
        (:Is%20Not%20Valid
          _)))
    (:Is%20Not%20Valid
      _))
  (bind _pinusclass (CallFunction|NumtoPinusClass (Variables|Default|GetnumSelectedPinus)))
  (bind _returnvalue (Game|SpawnActorfromClass _pinusclass (Math|Transform|MakeTransform (Transformation|GetWorldLocation (Variables|Default|GetpinusSpawnPoint)) "0, 0, 0" "0.100000,0.100000,0.100000") "AlwaysSpawn" "MultiplyWithRoot" 0 0))
  (Variables|Default|Setref_bp_pinus (Utilities|ResolveSoftReference _returnvalue))
  (Variables|Default|SetpinusIsCreated true)
  (Variables|Default|SetcanKick true)
  (bind _returnvalue_2 (Actor|GetActorOfClass "/Game/objects/camera/BP_Camera.BP_Camera_C"))
  (Default|RefreshPinus _returnvalue_2))

(event Input|EnhancedActionEvents|EnhancedInputActionIA_ChargeKick
  (params (ActionValue :type Boolean) (ElapsedSeconds :type Float%20%28double-precision%29) (TriggeredSeconds :type Float%20%28double-precision%29) (InputAction :type Input%20Action%20Object%20Reference :default "/Game/inputs/IA_ChargeKick.IA_ChargeKick"))
  (bind _charge (Variables|Default|Getcharge))
  ;[0 1 0] Запуска Charge
  (Rendering|SetVisibility _charge true false)
  (Components|Timeline|PlayfromStart _charge))

(event Input|EnhancedActionEvents|EnhancedInputActionIA_Kick
  (params (ActionValue :type Boolean) (ElapsedSeconds :type Float%20%28double-precision%29) (TriggeredSeconds :type Float%20%28double-precision%29) (InputAction :type Input%20Action%20Object%20Reference :default "/Game/inputs/IA_Kick.IA_Kick"))
  (bind _char (Variables|Default|Getchar))
  (bind _charge (Variables|Default|Getcharge))
  ;[0 1 1] Подготовка Pinus и Pirat к Pinus Kick
  (Audio|Components|Audio|Stop _charge)
  (Rendering|SetVisibility _charge false false)
  (bind _result (Math|Integer|IncrementInt (Class|PaperFlipbookComponent|GetPlaybackPositioninFrames _charge))
    (:%20%20
      (Variables|Default|SetkickPower _result)
      (Sprite|SetFlipbook _char "/Game/objects/pirat/attack.attack")
      (Components|Timeline|PlayfromStart _char)
      (Utilities|FlowControl|Delay 0.4)
      (CallFunction|KickPinus))))

(event Input|EnhancedActionEvents|EnhancedInputActionIA_UnbindPinus
  (params (ActionValue :type Boolean) (ElapsedSeconds :type Float%20%28double-precision%29) (TriggeredSeconds :type Float%20%28double-precision%29) (InputAction :type Input%20Action%20Object%20Reference :default "/Game/inputs/IA_UnbindPinus.IA_UnbindPinus"))
  ;[0 1 0] Отвязаться от Pinus
  (CallFunction|UnbindPinus))

(event Input|EnhancedActionEvents|EnhancedInputActionIA_PinusActivate
  (params (ActionValue :type Boolean) (ElapsedSeconds :type Float%20%28double-precision%29) (TriggeredSeconds :type Float%20%28double-precision%29) (InputAction :type Input%20Action%20Object%20Reference :default "/Game/inputs/IA_PinusActivate.IA_PinusActivate"))
  (bind _ref_bp_pinus (Variables|Default|Getref_bp_pinus))
  (bind _output (Utilities|ResolveSoftReference _ref_bp_pinus))
  ;[0 1 0] Активация Pinus
  (Utilities|IsValid _output
    (:Is%20Valid
      (Default|Activate _output))))

(event Input|EnhancedActionEvents|EnhancedInputActionIA_FlipPirat
  (params (ActionValue :type Boolean) (ElapsedSeconds :type Float%20%28double-precision%29) (TriggeredSeconds :type Float%20%28double-precision%29) (InputAction :type Input%20Action%20Object%20Reference :default "/Game/inputs/IA_FlipPirat.IA_FlipPirat"))
  ;[0 1 0] Разворот Pirat
  (CallFunction|UnbindPinus)
  (Pawn|SetControlRotation (Pawn|GetController) (Math|Rotator|SelectRotator "0.000000,180.000000,0.000000" "0, 0, 0" (== (.yaw (Pawn|GetControlRotation :!class /Script/Engine.Pawn)) 0.0))))

(event EventBeginPlay
  (bind _charge (Variables|Default|Getcharge))
  ;[1 1 0] Начальная настройка анимаций
  (Audio|Components|Audio|Stop _charge)
  (Rendering|SetVisibility _charge false false)
  (Components|Timeline|SetLooping _charge false)
  (Components|Timeline|SetLooping (Variables|Default|Getchar) false))

(fn ConstructionScript)

(fn KickPinus
  (bind _kickpower (Variables|Default|GetkickPower))
  (bind _kofkickpower (Variables|Default|GetkofKickPower))
  ;[0 1 1] Pinus Kick
  ; Определяем все Pinus в области пинка, удаляем им Arrow
  ; Определяем вектор импульса, умножаем на Charge и задаем импульс всем Pinus в области
  (bind _outactors (Actor|GetAllActorsOfClass "/Game/objects/arrow/BP_Arrow.BP_Arrow_C"))
  (for _array_element _outactors
    (Actor|DestroyActor _array_element))
  (for _array_element_2 (Collision|GetOverlappingActors (Variables|Default|GetboxAttack) "/Game/objects/pinus/BP_Pinus.BP_Pinus_C" :!class /Script/Engine.PrimitiveComponent)
    (bind _asbp_pinus (Utilities|Casting|CastToBP_Pinus _array_element_2))
    (Variables|/Game/objects/pinus/BP_Pinus.BP_Pinus_C|SetisKicked _asbp_pinus true)
    (Physics|AddImpulse (Variables|/Game/objects/pinus/BP_Pinus.BP_Pinus_C|GetCapsule _asbp_pinus) (Math|Vector|MakeVector (* _kickpower _kofkickpower (Math|Trig|Cos(Degrees) (Math|Float|SelectFloat (.pitch (Math|Rotator|FindLookatRotation (Transformation|GetWorldLocation (Variables|/Game/objects/pinus/BP_Pinus.BP_Pinus_C|GetCapsule _asbp_pinus)) (.location (.HitResult (Game|Player|GetHitResultUnderCursorbyChannel (Game|GetPlayerController 0) "TraceTypeQuery3" true))))) (- 1.8e+02 (.pitch (Math|Rotator|FindLookatRotation (Transformation|GetWorldLocation (Variables|/Game/objects/pinus/BP_Pinus.BP_Pinus_C|GetCapsule _asbp_pinus)) (.location (.HitResult (Game|Player|GetHitResultUnderCursorbyChannel (Game|GetPlayerController 0) "TraceTypeQuery3" true)))))) (== (.yaw (Pawn|GetControlRotation :!class /Script/Engine.Pawn)) 0.0)))) 0.0 (* _kickpower _kofkickpower (Math|Trig|Sin(Degrees) (Math|Float|SelectFloat (.pitch (Math|Rotator|FindLookatRotation (Transformation|GetWorldLocation (Variables|/Game/objects/pinus/BP_Pinus.BP_Pinus_C|GetCapsule _asbp_pinus)) (.location (.HitResult (Game|Player|GetHitResultUnderCursorbyChannel (Game|GetPlayerController 0) "TraceTypeQuery3" true))))) (- 1.8e+02 (.pitch (Math|Rotator|FindLookatRotation (Transformation|GetWorldLocation (Variables|/Game/objects/pinus/BP_Pinus.BP_Pinus_C|GetCapsule _asbp_pinus)) (.location (.HitResult (Game|Player|GetHitResultUnderCursorbyChannel (Game|GetPlayerController 0) "TraceTypeQuery3" true)))))) (== (.yaw (Pawn|GetControlRotation :!class /Script/Engine.Pawn)) 0.0))))) "None" false)
    (Development|PrintString (Utilities|String|ToString(Float) (* _kickpower _kofkickpower (Math|Trig|Cos(Degrees) (Math|Float|SelectFloat (.pitch (Math|Rotator|FindLookatRotation (Transformation|GetWorldLocation (Variables|/Game/objects/pinus/BP_Pinus.BP_Pinus_C|GetCapsule _asbp_pinus)) (.location (.HitResult (Game|Player|GetHitResultUnderCursorbyChannel (Game|GetPlayerController 0) "TraceTypeQuery3" true))))) (- 1.8e+02 (.pitch (Math|Rotator|FindLookatRotation (Transformation|GetWorldLocation (Variables|/Game/objects/pinus/BP_Pinus.BP_Pinus_C|GetCapsule _asbp_pinus)) (.location (.HitResult (Game|Player|GetHitResultUnderCursorbyChannel (Game|GetPlayerController 0) "TraceTypeQuery3" true)))))) (== (.yaw (Pawn|GetControlRotation :!class /Script/Engine.Pawn)) 0.0))))))
    (Development|PrintString (Utilities|String|ToString(Float) (* _kickpower _kofkickpower (Math|Trig|Sin(Degrees) (Math|Float|SelectFloat (.pitch (Math|Rotator|FindLookatRotation (Transformation|GetWorldLocation (Variables|/Game/objects/pinus/BP_Pinus.BP_Pinus_C|GetCapsule _asbp_pinus)) (.location (.HitResult (Game|Player|GetHitResultUnderCursorbyChannel (Game|GetPlayerController 0) "TraceTypeQuery3" true))))) (- 1.8e+02 (.pitch (Math|Rotator|FindLookatRotation (Transformation|GetWorldLocation (Variables|/Game/objects/pinus/BP_Pinus.BP_Pinus_C|GetCapsule _asbp_pinus)) (.location (.HitResult (Game|Player|GetHitResultUnderCursorbyChannel (Game|GetPlayerController 0) "TraceTypeQuery3" true)))))) (== (.yaw (Pawn|GetControlRotation :!class /Script/Engine.Pawn)) 0.0))))))))

(fn NumtoPinusClass
  (params (num :type Integer))
  ;[1 1 1] Принимаем индекс Pinus, возвращаем класс Pinus
  (switch int num
    (:Default
      _)
    (:0
      _)
    (:1
      (return "/Game/objects/pinus/BP_HellPinus.BP_HellPinus_C"))
    (:2
      (return "/Game/objects/pinus/BP_MagnetPinus.BP_MagnetPinus_C"))
    (:3
      (return "/Game/objects/pinus/BP_SpikePinus.BP_SpikePinus_C"))
    (:4
      (return "/Game/objects/pinus/BP_HolyPinus.BP_HolyPinus_C")))
  (return "/Game/objects/pinus/BP_Pinus.BP_Pinus_C"))

(fn UnbindPinus
  (bind _ref_bp_pinus (Variables|Default|Getref_bp_pinus))
  (bind _output (Utilities|ResolveSoftReference _ref_bp_pinus))
  (bind _bp_arrow (Variables|/Game/objects/pinus/BP_Pinus.BP_Pinus_C|Getbp_arrow _output))
  ;[1 1 1] Убираем разрешения, удаляем стрелку
  (Variables|Default|SetpinusIsCreated false)
  (Variables|Default|SetcanKick false)
  (Utilities|IsValid _output
    (:Is%20Valid
      (Utilities|IsValid _bp_arrow
        (:Is%20Valid
          (Actor|DestroyActor _bp_arrow))))))