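; BP_Pinus is a kickable object with a limited number of activations.
; On BeginPlay it spawns a scaled-down BP_Arrow at its own location and keeps a reference to it.
; Its Activate function succeeds only while it is flagged as kicked and has activations left, decrementing the count and returning whether activation happened.
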(event EventBeginPlay
  ;[1 1 0] Создание стрелки
  (bind _returnvalue (Game|SpawnActorfromClass "/Game/objects/arrow/BP_Arrow.BP_Arrow_C" (Math|Transform|MakeTransform (Transformation|GetActorLocation) "0, 0, 0" "0.100000,0.100000,0.100000") "AlwaysSpawn" "MultiplyWithRoot" 0 0))
  (Variables|Default|Setbp_arrow _returnvalue))

(event Collision|EventActorBeginOverlap
  (params (OtherActor :type Actor%20Object%20Reference)))

(event EventTick
  (params (DeltaSeconds :type Float%20%28single-precision%29)))

(fn ConstructionScript)

(fn Activate
  ;[1 1 1] Проверка возможности активации Pinus
  ; В зависимости от количества активаций и статуса пнутости
  (if (and (> (Variables|Default|GetactivationsCount) 0) (Variables|Default|GetisKicked))
    (bind _result (Math|Integer|DecrementInt (Variables|Default|GetactivationsCount))
      (:%20%20
        (Variables|Default|SetactivationsCount _result)
        (return true)))
    (else
      (return false))))