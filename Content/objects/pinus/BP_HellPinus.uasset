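; Hell variant of a pinus object that is meant to grow in size when activated.
; Its Activate override calls the parent first and, only if that succeeds, runs AddActorWorldTransform with an enlarged delta scale and passes the result on.
; An author note questions why the enlargement fails on repeated activations.
; BeginPlay and construction only call the parent.
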(event EventBeginPlay
  (|CallParentFunction))

(event Collision|EventActorBeginOverlap
  (params (OtherActor :type Actor%20Object%20Reference))
  (|CallParentFunction OtherActor) ; This node is disabled and will not be called.\nDrag off pins to build functionality.
)

(event EventTick
  (params (DeltaSeconds :type Float%20%28single-precision%29))
  (|CallParentFunction DeltaSeconds) ; This node is disabled and will not be called.\nDrag off pins to build functionality.
)

(fn ConstructionScript
  (|CallParentFunction))

(fn Activate
  ;[1 0 1] Увеличиваем размерчик
  ; Вопрос, почему это не срабатыывет несколько раз хммммм
  (bind _activated (|CallParentFunction))
  (if _activated
    (Class|Actor|AddActorWorldTransform (Math|Transform|MakeTransform "0, 0, 0" "0, 0, 0" "3.000000,3.000000,3.000000") false false)
    (return _activated)))