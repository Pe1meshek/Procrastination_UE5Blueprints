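; Magnet variant of a pinus object that, when activated, briefly pulls overlapping BP_Delo actors toward itself.
; Activate runs the parent activation, then enables the MagnetPole sphere at maximum radius, plays the Explosion flipbook and starts a looping per-frame timer.
; MagnetPoleAction shrinks the sphere in step with the flipbook's duration, applying distance-scaled impulses to overlapping Delo boxes.
; Once the radius nears zero, it clears the timer and hides and disables the field.
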(event EventBeginPlay
  ;[1 0 1] Прячем/отключаем все ненужное
  (|CallParentFunction)
  (Collision|SetCollisionEnabled (Variables|Default|GetmagnetPole) "NoCollision")
  (Rendering|SetVisibility (Variables|Default|Getexplosion) false false))

(event Collision|EventActorBeginOverlap
  (params (OtherActor :type Actor%20Object%20Reference))
  (|CallParentFunction OtherActor) ; This node is disabled and will not be called.\nDrag off pins to build functionality.
)

(event EventTick
  (params (DeltaSeconds :type Float%20%28single-precision%29))
  (|CallParentFunction DeltaSeconds) ; This node is disabled and will not be called.\nDrag off pins to build functionality.
)

(fn ConstructionScript
  (|CallParentFunction))

(fn Activate
  (bind _magnetpole (Variables|Default|GetmagnetPole))
  (bind _explosion (Variables|Default|Getexplosion))
  ;[1 0 1] Заряжаем радиус поля и включаем нужное
  ; Запускаем функцию изменения радиуса
  (bind _activated (|CallParentFunction))
  (if _activated
    (Utilities|IsValid _magnetpole
      (:Is%20Valid
        (Collision|SetCollisionEnabled _magnetpole "QueryAndPhysics")
        (Components|Sphere|SetSphereRadius _magnetpole (Variables|Default|GetmagnetPoleMaxRadius) true)
        (Utilities|IsValid _explosion
          (:Is%20Valid
            (Rendering|SetVisibility _explosion true false)
            (Components|Timeline|PlayfromStart _explosion)
            (bind _returnvalue (Utilities|Time|SetTimerbyEvent (EventDispatchers|CreateEvent :!event MagnetPoleAction) (Utilities|Time|GetWorldDeltaSeconds) true true))
            (Variables|Default|SetmagnetPoleTimerHandler _returnvalue))
          (:Is%20Not%20Valid
            _)))))
  (return _activated))

(fn MagnetPoleAction
  (bind _returnvalue (Utilities|Time|GetWorldDeltaSeconds))
  (bind _magnetpole (Variables|Default|GetmagnetPole))
  (bind _explosion (Variables|Default|Getexplosion))
  (bind _magnetpolemaxradius (Variables|Default|GetmagnetPoleMaxRadius))
  (bind _returnvalue_2 (Class|PaperFlipbookComponent|GetFlipbookLengthinFrames _explosion))
  (bind _returnvalue_3 (Class|PaperFlipbookComponent|GetFlipbookFramerate _explosion))
  (bind _sphereradius (Variables|/Script/Engine.SphereComponent|GetSphereRadius _magnetpole))
  (bind _returnvalue_4 (/ 1.0 _returnvalue_3))
  (bind _returnvalue_5 (* _returnvalue_4 _returnvalue_2))
  (bind _returnvalue_6 (/ _returnvalue_5 _returnvalue))
  (bind _returnvalue_7 (/ _magnetpolemaxradius _returnvalue_6))
  (bind _returnvalue_8 (- _sphereradius _returnvalue_7))
  ;[1 0 1] Уменьшаем радиус
  ; Если радиус не маловат, то ищем Delo в перечесении и тянем его к себе
  (Utilities|IsValid _magnetpole
    (:Is%20Valid
      (Components|Sphere|SetSphereRadius _magnetpole _returnvalue_8 true)
      (if (< _returnvalue_8 2.0)
        (Utilities|Time|ClearandInvalidateTimerbyHandle (Variables|Default|GetmagnetPoleTimerHandler))
        (Collision|SetCollisionEnabled (Variables|Default|GetmagnetPole) "NoCollision")
        (Rendering|SetVisibility _explosion false false)
        (else
          (for _array_element (Collision|GetOverlappingActors _magnetpole "/Game/objects/delo/BP_Delo.BP_Delo_C" :!class /Script/Engine.PrimitiveComponent)
            (bind _asbp_delo (Utilities|Casting|CastToBP_Delo _array_element))
            (Physics|AddImpulse (Variables|/Game/objects/delo/BP_Delo.BP_Delo_C|GetBox _asbp_delo) (* (- (Transformation|GetActorLocation) (Transformation|GetActorLocation _asbp_delo)) 20) "None" false)))))))