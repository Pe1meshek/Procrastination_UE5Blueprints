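; BP_SpikePinus is a Pinus variant that bursts into a radial spray of small Pinus actors when activated.
; Its Activate override runs the parent logic first and, on success, spawns NumOfSpawnPinus scaled-down copies of BP_Pinus evenly around itself in the XZ plane.
; Each spawn gets a heavier capsule mass scale, loses its BpArrow and receives an outward impulse along its angle.
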(event EventBeginPlay
  (|CallParentFunction) ; This node is disabled and will not be called.\nDrag off pins to build functionality.
)

(event Collision|EventActorBeginOverlap
  (params (OtherActor :type Actor%20Object%20Reference))
  (|CallParentFunction OtherActor) ; This node is disabled and will not be called.\nDrag off pins to build functionality.
)

(event EventTick
  (params (DeltaSeconds :type Float%20%28single-precision%29))
  (|CallParentFunction DeltaSeconds) ; This node is disabled and will not be called.\nDrag off pins to build functionality.
)

(fn ConstructionScript
  (|CallParentFunction))

(fn Activate
  (bind _returnvalue (Transformation|GetActorLocation))
  (bind _numofspawnpinus (Variables|Default|GetnumOfSpawnPinus))
  ;[1 0.5 0] Спавним Pinus вокруг и задаем им импульс
  (bind _activated (|CallParentFunction))
  (if _activated
    (for _index (range 0 _numofspawnpinus)
      (bind _returnvalue_2 (Game|SpawnActorfromClass "/Game/objects/pinus/BP_Pinus.BP_Pinus_C" (Math|Transform|MakeTransform (Math|Vector|MakeVector (+ (.x _returnvalue) (* (Math|Trig|Cos(Degrees) (* _index (/ 3.6e+02 (Math|Conversions|ToFloat(Integer) _numofspawnpinus)))) 5e+01)) (.y _returnvalue) (+ (.z _returnvalue) (* (Math|Trig|Sin(Degrees) (* _index (/ 3.6e+02 (Math|Conversions|ToFloat(Integer) _numofspawnpinus)))) 5e+01))) (Math|Rotator|MakeRotator 0.0 (* _index (/ 3.6e+02 (Math|Conversions|ToFloat(Integer) _numofspawnpinus))) 0.0) "0.100000,0.100000,0.100000") "AlwaysSpawn" "MultiplyWithRoot" 0 0))
      (Class|PrimitiveComponent|SetMassScale (Variables|/Game/objects/pinus/BP_Pinus.BP_Pinus_C|GetCapsule _returnvalue_2) "None" 5.0)
      (Actor|DestroyActor (Variables|/Game/objects/pinus/BP_Pinus.BP_Pinus_C|Getbp_arrow _returnvalue_2))
      (Physics|AddImpulse (Variables|/Game/objects/pinus/BP_Pinus.BP_Pinus_C|GetCapsule _returnvalue_2) (Math|Vector|MakeVector (* (Math|Trig|Cos(Degrees) (* _index (/ 3.6e+02 (Math|Conversions|ToFloat(Integer) _numofspawnpinus)))) 5e+02) 0.0 (* (Math|Trig|Sin(Degrees) (* _index (/ 3.6e+02 (Math|Conversions|ToFloat(Integer) _numofspawnpinus)))) 5e+02)) "None" false))
    (return _activated)))