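; BP_Deadline is a moving hazard that ends the game when it catches a key object.
; Each Tick offsets its Cube by a tenth of the Speed vector without sweep, not scaled by delta time.
; An overlapping BP_Pinus is destroyed, and the BP_Pirat found by class lookup has its CanKick and PinusIsCreated flags cleared.
; Overlapping BP_Delo, BP_Varp or BP_Pirat pauses the game and shows the WB_Lose widget.
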(event EventBeginPlay)

(event Collision|EventActorBeginOverlap
  (params (OtherActor :type Actor%20Object%20Reference))
  ;[1 1 1] Удаление Pinus или gameover если deadline настигла один из ключевых объектов
  (bind _asbp_pinus (Utilities|Casting|CastToBP_Pinus OtherActor)
    (:then
      (Actor|DestroyActor _asbp_pinus)
      (bind _returnvalue (Actor|GetActorOfClass "/Game/objects/pirat/BP_Pirat.BP_Pirat_C"))
      (Variables|/Game/objects/pirat/BP_Pirat.BP_Pirat_C|SetcanKick _returnvalue false)
      (Variables|/Game/objects/pirat/BP_Pirat.BP_Pirat_C|SetpinusIsCreated _returnvalue false))
    (:CastFailed
      (Utilities|Casting|CastToBP_Delo OtherActor
        (:then
          _)
        (:CastFailed
          (Utilities|Casting|CastToBP_Varp OtherActor
            (:then
              _)
            (:CastFailed
              (Utilities|Casting|CastToBP_Pirat OtherActor)))))
      (Game|SetGamePaused true)
      (bind _returnvalue_2 (UserInterface|CreateWidget "/Game/Widgets/WB_Lose.WB_Lose_C"))
      (UserInterface|Viewport|AddtoViewport _returnvalue_2 0))))

(event EventTick
  (params (DeltaSeconds :type Float%20%28single-precision%29))
  ;[1 1 1] Движение в заданном векторе
  (Transformation|AddWorldOffset (Variables|Default|GetCube) (* (Variables|Default|Getspeed) 0.1) false false))

(fn ConstructionScript)